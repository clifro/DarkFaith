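; BP_Hero is a side-scrolling Paper2D player character that runs and jumps along the world X axis.
; The Forward axis drives movement, flips the sprite's yaw to face the input, and picks idle, run, jump or fall flipbooks from movement state and velocity.
; While grounded, Tick traces downward against static geometry and pitches the sprite to the surface normal, inverting the pitch when facing the other way.
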(event `self.ReceiveTick`
  (params (DeltaSeconds :type "Float (single-precision)"))
  (bind _returnvalue (`self.K2_GetActorLocation`))
  (bind _sprite (`self.Sprite`))
  (bind (_returnvalue_roll _returnvalue_pitch _returnvalue_yaw) (`KismetMathLibrary.BreakRotator` (`SceneComponent.K2_GetComponentRotation` _sprite)))
  (if (not (`NavMovementComponent.IsFalling` (`self.CharacterMovement`)))
    (bind _outhit (`KismetSystemLibrary.LineTraceSingleForObjects` _returnvalue (+ _returnvalue (* (`self.GetActorUpVector`) -100.0)) (`|MakeArray` "ObjectTypeQuery1" :!type "EObjectTypeQuery Enum") false (`|MakeArray` self :!type "Actor Object Reference")))
    (bind (_returnvalue_roll_2 _returnvalue_pitch_2) (`KismetMathLibrary.BreakRotator` (`KismetMathLibrary.MakeRotFromYZ` (`self.GetActorRightVector`) (`.ImpactNormal` (`GameplayStatics.BreakHitResult` _outhit)))))
    (`SceneComponent.K2_SetWorldRotation` _sprite (`KismetMathLibrary.MakeRotator` _returnvalue_roll (* _returnvalue_pitch_2 (select `bool` (== (`self.Rotation`) 0.0) :`false` -1.0 :`true` 1.0)) _returnvalue_yaw) false false)))

(event `InputAxis|Forward`
  (params (AxisValue :type "Float (single-precision)"))
  (bind _sprite (`self.Sprite`))
  (bind (_velocity_x _velocity_y _velocity_z) (`KismetMathLibrary.BreakVector` (`MovementComponent.Velocity` (`self.CharacterMovement`))))
  (bind _output_get (set `self.Rotation` (`KismetMathLibrary.SelectFloat` 180.0 (select `bool` (>= AxisValue 1.0) :`false` (`self.Rotation`)) (<= AxisValue -1.0))))
  (`SceneComponent.K2_SetWorldRotation` (`self.Sprite`) (`KismetMathLibrary.MakeRotator` 0.0 0.0 _output_get) false false)
  (`PawnMovementComponent.AddInputVector` (`self.CharacterMovement`) (`KismetMathLibrary.MakeVector` AxisValue) false)
  (if (`NavMovementComponent.IsFalling` (`self.CharacterMovement`))
    (if (> _velocity_z 0.0)
      (`PaperFlipbookComponent.SetFlipbook` _sprite "/Game/FlibBook/Hero/FB_Hero_Jump.FB_Hero_Jump")
      (else
        (`PaperFlipbookComponent.SetFlipbook` _sprite "/Game/FlibBook/Hero/FB_Hero_Fall.FB_Hero_Fall")))
    (elif (> (`KismetMathLibrary.Abs` _velocity_x) 0.0)
      (`PaperFlipbookComponent.SetFlipbook` _sprite "/Game/FlibBook/Hero/FB_Hero_Run.FB_Hero_Run")
      (else
        (`PaperFlipbookComponent.SetFlipbook` _sprite "/Game/FlibBook/Hero/FB_Hero_Idle.FB_Hero_Idle")))))

(event `InputAction|Jump`
  (params (Key :type "Key Structure"))
  (:`Pressed`
    (`self.Jump`)))

(fn `UserConstructionScript`)