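; BP_Hero1 is a 2D flipbook hero character in which only the Jump input is functional.
; The Forward axis, BeginPlay and Tick events are empty.
; Disconnected logic would move and flip the sprite, choose idle, run, jump or fall flipbooks from movement state, and pitch the sprite to ground slopes using a downward line trace, but none of it runs.
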(event `self.ReceiveTick`
  (params (DeltaSeconds :type "Float (single-precision)")))

(event `InputAxis|Forward`
  (params (AxisValue :type "Float (single-precision)")))

(event `InputAction|Jump`
  (params (Key :type "Key Structure"))
  (:`Pressed`
    (`self.Jump`)))

(fn `UserConstructionScript`)