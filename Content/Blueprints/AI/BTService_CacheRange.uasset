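; Behavior tree service that caches the AI pawn's range to a character in the blackboard.
; On each tick it casts the owner to AI_CharacterController and searches the world for all BP_Character_Base actors.
; If any exist, it writes the controlled pawn's distance to the first one found into the Distance float key, without filtering or sorting the results.
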(event `self.ReceiveTick`
  (params (OwnerActor :type "Actor Object Reference") (DeltaSeconds :type "Float (single-precision)"))
  (bind _asai_character_controller (cast `/Game/Blueprints/AI/AI_CharacterController` OwnerActor))
  (bind _outactors (`GameplayStatics.GetAllActorsOfClass` "/Game/Blueprints/Characters/BP_Character_Base.BP_Character_Base_C"))
  (if (> (`KismetArrayLibrary.Array_Length` _outactors) 0)
    (`BlackboardComponent.SetValueAsFloat` (`AIBlueprintHelperLibrary.GetBlackboard` OwnerActor) "Distance" (`Actor.GetDistanceTo` (`Controller.K2_GetPawn` _asai_character_controller) (`|GetArrayItem` _outactors)))))