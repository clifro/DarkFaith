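; Behavior tree decorator that gates a branch on whether the AI's controlled pawn is within a short, hardcoded range of the hero.
; PerformConditionCheck casts the owner to AI_CharacterController and measures the distance from its pawn to the first BP_CharacterHero returned by GetAllActorsOfClass on each check.
; It fails when the cast fails or no hero exists.
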(fn `PerformConditionCheck`
  (params (OwnerActor :type "Actor Object Reference"))
  (returns (ReturnValue :type Boolean))
  (bind _asai_character_controller (cast `/Game/Blueprints/AI/AI_CharacterController` OwnerActor)
    (:`then`
      (bind _outactors (`GameplayStatics.GetAllActorsOfClass` "/Game/Blueprints/Characters/BP_CharacterHero.BP_CharacterHero_C"))
      (if (> (`KismetArrayLibrary.Array_Length` _outactors) 0)
        (return (<= (`Actor.GetDistanceTo` (`Controller.K2_GetPawn` _asai_character_controller) (`|GetArrayItem` _outactors)) 80.0))
        (else
          _)))
    (:`CastFailed`
      _))
  (return false))