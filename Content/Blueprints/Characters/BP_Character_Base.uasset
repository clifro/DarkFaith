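; Base 2D sprite character with light/heavy attack inputs and slope-aware sprite placement.
; PerformAttack box-traces forward from the sprite, damaging each actor once until the sprite's animation finishes and clears the hit list.
; While grounded, Tick raycasts at two feet to pitch the sprite along the slope, then offsets its height trigonometrically from the foot surface normals.
; While falling, sprite pitch resets to zero.
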(event `InputAction|HeavyAttack`
  (params (Key :type "Key Structure"))
  (:`Pressed`
    (`self.Attack` "HeavyAttack")))

(event `self.ReceiveBeginPlay`
  (`parent.ReceiveBeginPlay`)
  (add `PaperFlipbookComponent.OnFinishedPlaying` (`self.Sprite`) (delegate `AttackDone`))
  (set `self.SpriteRelativeLoc` (`SceneComponent.RelativeLocation` (`self.Sprite`))))

(event `InputAction|Attack`
  (params (Key :type "Key Structure"))
  (:`Pressed`
    (`self.Attack` "LightAttack")))

(event `AttackDone`
  (`BlueprintSetLibrary.Set_Clear` (`self.HitActors`)))

(event `self.PerformAttack`
  (params (Range :type "Float (single-precision)") (Damage :type "Float (single-precision)"))
  (bind _sprite (`self.Sprite`))
  (bind _returnvalue (`SceneComponent.K2_GetComponentLocation` _sprite))
  (bind _outhits (`KismetSystemLibrary.BoxTraceMultiForObjects` _returnvalue (+ _returnvalue (* (`SceneComponent.GetForwardVector` _sprite) Range)) (0.0 10.0 25.0) (struct) (`self.Object Types`) false (`|MakeArray` self :!type "Actor Object Reference") "None" true (struct :`R` 1.0 :`A` 1.0) (struct :`G` 1.0 :`A` 1.0) 0.5))
  (for _array_element _outhits
    (bind (_bblockinghit _binitialoverlap _time _distance _location _impactpoint _normal _impactnormal _physmat _hitactor) (`GameplayStatics.BreakHitResult` _array_element))
    (if (not (`BlueprintSetLibrary.Set_Contains` (`self.HitActors`) _hitactor))
      (`BlueprintSetLibrary.Set_Add` (`self.HitActors`) _hitactor)
      (`GameplayStatics.ApplyDamage` _hitactor Damage))))

(event `self.ReceiveTick`
  (params (DeltaSeconds :type "Float (single-precision)"))
  (bind _sprite (`self.Sprite`))
  (bind (_returnvalue_roll _returnvalue_pitch _returnvalue_yaw) (`KismetMathLibrary.BreakRotator` (`SceneComponent.K2_GetComponentRotation` _sprite)))
  (`parent.ReceiveTick` DeltaSeconds)
  (if (`NavMovementComponent.IsFalling` (`self.CharacterMovement`))
    (`SceneComponent.K2_SetWorldRotation` _sprite (`KismetMathLibrary.MakeRotator` _returnvalue_roll 0.0 _returnvalue_yaw) false false)
    (else
      (bind (_impactpoint _impactnormal) (`self.GetFootRayCast` (`self.Foot1Depth`) (`self.Foot1Distance`)))
      (bind (_impactpoint_2 _impactnormal_2) (`self.GetFootRayCast` (`self.Foot2Depth`) (`self.Foot2Distance`)))
      (`self.AlignToSlope` _impactpoint _impactpoint_2 _impactnormal _impactnormal_2)
      (`self.Adjust Height Based on Slope` _impactpoint _impactnormal _impactpoint_2 _impactnormal_2))))

(fn `Adjust Height Based on Slope`
  (params (Foot1Loc :type "Vector Structure") (Foot1Normal :type "Vector Structure") (Foot2Loc :type "Vector Structure") (Foot2Normal :type "Vector Structure"))
  (bind _returnvalue (`self.GetActorRightVector`))
  (bind (_returnvalue_roll _returnvalue_pitch) (`KismetMathLibrary.BreakRotator` (`self.K2_GetActorRotation`)))
  (bind _foot1normal (`local.Foot1Normal`))
  (bind _foot2normal (`local.Foot2Normal`))
  (bind (_spriterelativeloc_x _spriterelativeloc_y _spriterelativeloc_z) (`KismetMathLibrary.BreakVector` (`self.SpriteRelativeLoc`)))
  (bind _returnvalue_2 (`KismetMathLibrary.Normal` (- Foot1Loc Foot2Loc)))
  (`SceneComponent.K2_SetRelativeLocation` (`self.Sprite`) (+ (`KismetMathLibrary.MakeVector` 0.0 0.0 _spriterelativeloc_z) (* (`SceneComponent.GetUpVector` (`self.Sprite`)) (* (`KismetMathLibrary.SafeDivide` (`KismetMathLibrary.Vector_Distance` Foot1Loc Foot2Loc) (+ (`KismetMathLibrary.SafeDivide` 1.0 (`KismetMathLibrary.DegTan` (- 180.0 (`KismetMathLibrary.DegAcos` (`KismetMathLibrary.Dot_VectorVector` _returnvalue_2 (`KismetMathLibrary.Normal` (`KismetMathLibrary.Cross_VectorVector` (`local.Foot1Normal`) _returnvalue))))))) (`KismetMathLibrary.SafeDivide` 1.0 (`KismetMathLibrary.DegTan` (- 180.0 (`KismetMathLibrary.DegAcos` (`KismetMathLibrary.Dot_VectorVector` _returnvalue_2 (`KismetMathLibrary.Normal` (`KismetMathLibrary.Cross_VectorVector` (`local.Foot2Normal`) _returnvalue))))))))) (* (`KismetMathLibrary.SignOfFloat` (.x (`KismetMathLibrary.SelectVector` (- _foot1normal _foot2normal) (- _foot2normal _foot1normal) (== _returnvalue_pitch 0.0)))) -1.0)))) false false))

(fn `AlignToSlope`
  (params (Foot1 :type "Vector Structure") (Foot2 :type "Vector Structure") (Foot1Normal :type "Vector Structure") (Foot2Normal :type "Vector Structure"))
  (bind _returnvalue (`self.GetActorRightVector`))
  (bind _sprite (`self.Sprite`))
  (bind (_returnvalue_roll _returnvalue_pitch _returnvalue_yaw) (`KismetMathLibrary.BreakRotator` (`SceneComponent.K2_GetComponentRotation` _sprite)))
  (bind (_returnvalue_roll_2 _returnvalue_pitch_2) (`KismetMathLibrary.BreakRotator` (`KismetMathLibrary.MakeRotFromYZ` _returnvalue (`KismetMathLibrary.Cross_VectorVector` (`KismetMathLibrary.Normal` (- Foot1 Foot2)) _returnvalue))))
  (`SceneComponent.K2_SetWorldRotation` _sprite (`KismetMathLibrary.MakeRotator` _returnvalue_roll _returnvalue_pitch_2 _returnvalue_yaw) false false))

(fn `GetFootRayCast`
  (params (FootDepth :type "Float (double-precision)") (FootDistance :type "Float (double-precision)"))
  (returns (ImpactPoint :type "Vector Structure") (ImpactNormal :type "Vector Structure") (IsHit :type Boolean))
  (bind _sprite (`self.Sprite`))
  (bind _returnvalue (+ (+ (`SceneComponent.K2_GetComponentLocation` _sprite) (* (`SceneComponent.GetUpVector` _sprite) (`local.FootDepth`))) (* (`SceneComponent.GetForwardVector` (`self.Sprite`)) (`local.FootDistance`))))
  (bind (_outhit _returnvalue_2) (`KismetSystemLibrary.LineTraceSingleForObjects` (+ _returnvalue (0.0 0.0 0.0)) (+ _returnvalue (* (`self.GetActorUpVector`) -20.0)) (`|MakeArray` "ObjectTypeQuery1" :!type "EObjectTypeQuery Enum") false (`|MakeArray` self :!type "Actor Object Reference") "None" true (struct :`R` 1.0 :`A` 1.0) (struct :`G` 1.0 :`A` 1.0) 0.5))
  (bind (_bblockinghit _binitialoverlap _time _distance _location _impactpoint _normal _impactnormal) (`GameplayStatics.BreakHitResult` _outhit))
  (return _impactpoint _impactnormal _returnvalue_2))

(fn `UserConstructionScript`)