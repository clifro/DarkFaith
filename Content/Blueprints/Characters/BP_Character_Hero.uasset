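; BP_Character_Hero is a hero character Blueprint that shows its health on screen through a WB_HP widget.
; On BeginPlay it runs the parent logic, creates the widget, adds it to the viewport and binds to the OnHealthUpdated event dispatcher.
; Each health update passes Health divided by MaxHealth to the widget's SetHealth, so the display is event-driven with no Tick polling.
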(event `self.ReceiveBeginPlay`
  (`parent.ReceiveBeginPlay`)
  (bind _returnvalue (`|CreateWidget` "/Game/Blueprints/Widgets/WB_HP.WB_HP_C"))
  (bind _output_get (set `self.HPWidget` _returnvalue))
  (`UserWidget.AddToViewport` _output_get 0)
  (add `DFCharacterBase.OnHealthUpdated` (delegate `OnHealthUpdated_Event`)))

(event `OnHealthUpdated_Event`
  (params (Health :type "Float (single-precision)") (MaxHealth :type "Float (single-precision)"))
  (`/Game/Blueprints/Widgets/WB_HP.SetHealth` (`self.HPWidget`) (/ Health MaxHealth)))

(fn `UserConstructionScript`
  (`parent.UserConstructionScript`))